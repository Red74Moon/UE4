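; BP_MoveRect moves its Sphere component around a square path in relative space, bounded by zero and DestPos on X and Y.
; A looping 0.01-second timer replaces Tick and calls MoveRect, which switches on the MoveType state while IsPlay is true.
; Each direction function offsets the sphere by Speed times world delta seconds, not the timer interval, and sets the next state at its bound.
; The PressP interface event toggles IsPlay.
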(event `self.ReceiveTick`
  (params (DeltaSeconds :type "Float (single-precision)")))

(event `self.ReceiveBeginPlay`
  ;[1 1 1] Timer로 수정된 사각형 움직임
  (`KismetSystemLibrary.K2_SetTimer` null "MoveRect" 0.01 true))

(event `/Game/Class/BPI_PressP.PressP`
  ;[1 1 1] 인터페이스로 구성
  (set `self.IsPlay` (not (`self.IsPlay`))))

(fn `MoveBottom`
  (params (DelteSecond :type "Float (double-precision)"))
  (bind (_relativelocation_x _relativelocation_y) (`KismetMathLibrary.BreakVector` (`SceneComponent.RelativeLocation` (`self.Sphere`))))
  ;[1 1 1] 아래쪽
  (bind _result (`/Engine/EditorBlueprintResources/StandardMacros.NegateFloat` (* DelteSecond (`self.Speed`)))
    (:`  `
      (`SceneComponent.K2_AddRelativeLocation` (`self.Sphere`) (`KismetMathLibrary.MakeVector` 0.0 _result) false false)
      (if (< _relativelocation_y 0.0)
        (set `self.MoveType` "NewEnumerator0")))))

(fn `MoveLeft`
  (params (DelteSecond :type "Float (double-precision)"))
  (bind _relativelocation_x (`KismetMathLibrary.BreakVector` (`SceneComponent.RelativeLocation` (`self.Sphere`))))
  ;[1 1 1] 외쪽
  (bind _result (`/Engine/EditorBlueprintResources/StandardMacros.NegateFloat` (* DelteSecond (`self.Speed`)))
    (:`  `
      (`SceneComponent.K2_AddRelativeLocation` (`self.Sphere`) (`KismetMathLibrary.MakeVector` _result) false false)
      (if (< _relativelocation_x 0.0)
        (set `self.MoveType` "NewEnumerator3")))))

(fn `MoveRect`
  (bind _returnvalue (`GameplayStatics.GetWorldDeltaSeconds`))
  (if (`self.IsPlay`)
    (switch `/Game/Class/EN_MoveType` (`self.MoveType`)
      (:`NewEnumerator0`
        (`self.MoveRight` _returnvalue))
      (:`NewEnumerator1`
        (`self.MoveLeft` _returnvalue))
      (:`NewEnumerator2`
        (`self.MoveUp` _returnvalue))
      (:`NewEnumerator3`
        (`self.MoveBottom` _returnvalue)))))

(fn `MoveRight`
  (params (DeltaSecond :type "Float (double-precision)"))
  (bind _relativelocation_x (`KismetMathLibrary.BreakVector` (`SceneComponent.RelativeLocation` (`self.Sphere`))))
  ;[1 1 1] 오른쪽
  (`SceneComponent.K2_AddRelativeLocation` (`self.Sphere`) (`KismetMathLibrary.MakeVector` (* DeltaSecond (`self.Speed`))) false false)
  (if (> _relativelocation_x (`self.DestPos`))
    (set `self.MoveType` "NewEnumerator2")))

(fn `MoveUp`
  (params (DeltaSecond :type "Float (double-precision)"))
  (bind (_relativelocation_x _relativelocation_y) (`KismetMathLibrary.BreakVector` (`SceneComponent.RelativeLocation` (`self.Sphere`))))
  ;[1 1 1] 위쪽
  (`SceneComponent.K2_AddRelativeLocation` (`self.Sphere`) (`KismetMathLibrary.MakeVector` 0.0 (* DeltaSecond (`self.Speed`))) false false)
  (if (> _relativelocation_y (`self.DestPos`))
    (set `self.MoveType` "NewEnumerator1")))

(fn `UserConstructionScript`)