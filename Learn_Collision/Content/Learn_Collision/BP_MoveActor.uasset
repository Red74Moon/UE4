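; BP_MoveActor is a collision-learning actor whose Sphere slides back and forth along local X between two limits.
; PressP toggles movement, and Tick calls MoveSphere with DeltaSeconds only while Condition is true.
; BeginPlay binds to each ChangeColor actor's color dispatcher, and a generated handler sets Condition from the received color.
; Separate helpers check all colors, print a minute-second timer, add values and print hello.
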(event `/Game/Learn_Collision/BPI_PressP.PressP`
  ;[1 1 1] 인터페이스로 구성
  (set `self.IsMove` (not (`self.IsMove`))))

(event `self.ReceiveTick`
  (params (DeltaSeconds :type "Float (single-precision)"))
  (if (`self.Condition`)
    (`self.MoveSphere` DeltaSeconds)))

(event `self.ReceiveBeginPlay`
  (for _array_element (`self.ChangeColor`)
    (add `/Game/Learn_Collision/BP_ChangeColor.NewEventDispatcher_ChangeColor` _array_element (`|CreateDelegate` :!event `BP_MoveActor_AutoGenFunc`))))

(fn `Add APB`
  (params (A :type "Float (double-precision)") (B :type "Float (double-precision)"))
  (returns (Result :type "Float (double-precision)"))
  ;[1 1 1] 함수 생성하고 입력값 받아서 출력(퓨어로 만듬)
  (return (+ A B)))

(fn `BP_MoveActor_AutoGenFunc`
  (params (Color :type "/Game/Learn_Collision/Enum_Color Enum" :default "NewEnumerator0"))
  (if (`|EnumEquality` Color "NewEnumerator1")
    (set `self.Condition` true)
    (else
      (set `self.Condition` false))))

(fn `Check Color`
  (returns (IsAllColor :type Boolean))
  (for _array_element (`self.ChangeColor`)
    (if (not (`|EnumEquality` (`/Game/Learn_Collision/BP_ChangeColor.Color` _array_element) "NewEnumerator1"))
      (return false)))
  (return true))

(fn `CountTimer`
  (params (Aaa :type "Float (double-precision)"))
  (bind _returnvalue (* Aaa 1.0))
  ;[1 1 1] 시간 분-초 출력
  (bind _output_get (set `self.TotalDist` (+ _returnvalue (`self.TotalDist`))))
  (bind _returnvalue_2 (`KismetStringLibrary.Concat_StrStr` (`self.IntToString00` (`KismetMathLibrary.FFloor` (/ _output_get 60.0))) "분" (`self.IntToString00` (`KismetMathLibrary.FFloor` (mod _output_get 60.0))) "초"))
  ;[1 1 1] 앞시간과 다음시간이 같은지 검사해서 다른 경우에만 출력
  (if (`KismetStringLibrary.NotEqual_StrStr` (`self.OldTime`) _returnvalue_2)
    (bind _output_get_2 (set `self.OldTime` _returnvalue_2))
    (`KismetSystemLibrary.PrintString` _output_get_2 true true (struct :`G` 0.66 :`B` 1.0 :`A` 1.0) 1.0)
    (`self.K2_AddActorLocalOffset` (`KismetMathLibrary.MakeVector` _returnvalue))))

(fn `IntToString00`
  (params (DeltaSecond :type Integer))
  (returns (resultString :type String))
  ;[1 1 1] 00분00초 함수
  (if (< DeltaSecond 10)
    (return (`KismetStringLibrary.Concat_StrStr` "0" (`KismetStringLibrary.Conv_IntToString` DeltaSecond)))
    (else
      (return (`KismetStringLibrary.Conv_IntToString` DeltaSecond)))))

(fn `MoveSphere`
  (params (A :type "Float (double-precision)"))
  (bind _returnvalue (* A 100.0))
  (bind _sphere (`self.Sphere`))
  (bind _relativelocation_x (`KismetMathLibrary.BreakVector` (`SceneComponent.RelativeLocation` (`self.Sphere`))))
  (bind _relativelocation_x_2 (`KismetMathLibrary.BreakVector` (`SceneComponent.RelativeLocation` (`self.Sphere`))))
  ;[1 1 1] 'P'Key입력 여부 체크
  (if (`self.IsMove`)
    ;[1 1 1] 구체 오른쪽 왼쪽 반복 움직임
    (if (`self.IsRight`)
      ;;[1 1 1] 오른쪽
      (`SceneComponent.K2_AddLocalOffset` _sphere (`KismetMathLibrary.MakeVector` _returnvalue) false false)
      (if (> _relativelocation_x 200.0)
        (set `self.IsRight` false))
      (else
        ;;[1 1 1] 왼쪽
        (bind _result (`/Engine/EditorBlueprintResources/StandardMacros.NegateFloat` _returnvalue)
          (:`  `
            (`SceneComponent.K2_AddLocalOffset` _sphere (`KismetMathLibrary.MakeVector` _result) false false)
            (if (< _relativelocation_x_2 -200.0)
              (set `self.IsRight` true))))))))

(fn `PrintHello`
  ;[1 1 1] 에디터에서 호출
  (`self.PrintHello`))

(fn `PrintHelloBP`
  (`KismetSystemLibrary.PrintString` "HelloBP_MoveActor"))

(fn `UserConstructionScript`)