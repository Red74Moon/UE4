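; HUD Blueprint that creates the HUD widget on BeginPlay, switches to game-only input and hides the cursor.
; A looping timer accumulates time scaled by Speed into a five-minute countdown, updating the zero-padded minute/second text only when it changes.
; Wrapper functions forward coin count, score and menu display to the widget.
; Coin and score calls arriving before the widget exists are cached and retried by timer until it is valid.
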(event `self.ReceiveBeginPlay`
  (bind _returnvalue (`GameplayStatics.GetPlayerController` 0))
  (bind _returnvalue_2 (`|CreateWidget` "/Game/Learn_Collision/HudWidget.HudWidget_C"))
  (bind _output_get (set `self.HudWidget` _returnvalue_2))
  (`UserWidget.AddToViewport` _output_get 0)
  (`KismetSystemLibrary.K2_SetTimer` null "UpdateCountDown" 0.01 true)
  (`WidgetBlueprintLibrary.SetInputMode_GameOnly` _returnvalue)
  (set `PlayerController.bShowMouseCursor` false _returnvalue))

(fn `FloatToStr00`
  (params (num :type "Float (double-precision)"))
  (returns (Result :type String))
  (bind _returnvalue (`KismetMathLibrary.FFloor` num))
  (if (< _returnvalue 10)
    (return (`KismetStringLibrary.Concat_StrStr` "0" (`KismetStringLibrary.Conv_IntToString` _returnvalue)))
    (else
      (return (`KismetStringLibrary.Conv_IntToString` _returnvalue)))))

(fn `SetCoinCount`
  (params (Cur :type Integer) (Max :type Integer))
  (bind _hudwidget (`self.HudWidget`))
  (`/Engine/EditorBlueprintResources/StandardMacros.IsValid` _hudwidget
    (:`Is Valid`
      (`/Game/Learn_Collision/HudWidget.SetCoinCount` _hudwidget Cur Max))
    (:`Is Not Valid`
      (set `self.BackpCur` Cur)
      (set `self.BackupMax` Max)
      (`KismetSystemLibrary.K2_SetTimer` null "UpdateSetCoinCount" 0.1))))

(fn `SetTextScore`
  (params (Score :type Integer))
  (bind _hudwidget (`self.HudWidget`))
  (`/Engine/EditorBlueprintResources/StandardMacros.IsValid` _hudwidget
    (:`Is Valid`
      (`/Game/Learn_Collision/HudWidget.SetTextScore` _hudwidget Score))
    (:`Is Not Valid`
      (set `self.BackupScore` Score)
      (`KismetSystemLibrary.K2_SetTimer` null "UpdateTextScore" 0.1))))

(fn `SetTimeText`
  (params (InString :type String))
  (set `/Game/Learn_Collision/HudWidget.TimeText` (`KismetTextLibrary.Conv_StringToText` InString) (`self.HudWidget`)))

(fn `ShowMenu`
  (`/Game/Learn_Collision/HudWidget.ShowMenu` (`self.HudWidget`)))

(fn `UpdateCountDown`
  ;[1 1 1] 초단위 누적
  (bind _output_get (set `self.TotalSec` (+ (* (`self.Speed`) 0.01) (`self.TotalSec`))))
  (bind _returnvalue (`KismetMathLibrary.FClamp` (- 300.0 _output_get) 0.0 300.0))
  (bind _returnvalue_2 (`KismetStringLibrary.Concat_StrStr` (`self.FloatToStr00` (/ _returnvalue 60.0)) "분" (`self.FloatToStr00` (mod _returnvalue 60.0)) "초"))
  ;[1 1 1] Str 출력
  (if (`KismetStringLibrary.NotEqual_StrStr` _returnvalue_2 (`self.BeforStr`))
    (set `/Game/Learn_Collision/HudWidget.TimeText` (`KismetTextLibrary.Conv_StringToText` _returnvalue_2) (`self.HudWidget`))
    (set `self.BeforStr` _returnvalue_2)))

(fn `UpdateSetCoinCount`
  (bind _hudwidget (`self.HudWidget`))
  (`/Engine/EditorBlueprintResources/StandardMacros.IsValid` _hudwidget
    (:`Is Valid`
      (`/Game/Learn_Collision/HudWidget.SetCoinCount` _hudwidget (`self.BackpCur`) (`self.BackupMax`)))
    (:`Is Not Valid`
      (`KismetSystemLibrary.K2_SetTimer` null "UpdateSetCoinCount" 0.1))))

(fn `UpdateTextScore`
  (bind _hudwidget (`self.HudWidget`))
  (`/Engine/EditorBlueprintResources/StandardMacros.IsValid` _hudwidget
    (:`Is Valid`
      (`/Game/Learn_Collision/HudWidget.SetTextScore` _hudwidget (`self.BackupScore`)))
    (:`Is Not Valid`
      (`KismetSystemLibrary.K2_SetTimer` null "UpdateTextScore" 0.1))))

(fn `UserConstructionScript`)