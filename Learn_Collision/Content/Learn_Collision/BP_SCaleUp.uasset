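; BP_SCaleUp is a collision-learning actor that grows its Cube based on which coins in its Coin array are hidden.
; On BeginPlay it binds a delegate to each coin's hidden event dispatcher, presumably targeting ScaleUp.
; ScaleUp rescans the whole array, incrementing NewScale3D for every hidden coin and applying it as the Cube's relative scale.
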(event `self.ReceiveBeginPlay`
  (for _array_element (`self.Coin`)
    (add `/Game/Learn_Collision/BP_Coin.NewEventDispatcher_Hidden` _array_element (`|CreateDelegate` :!event `ScaleUp`))))

(fn `ScaleUp`
  (bind _new_scale_3d (`self.New Scale 3D`))
  (for _array_element (`self.Coin`)
    (if (`Actor.bHidden` _array_element)
      (set `self.New Scale 3D` (+ _new_scale_3d 1.0))
      (`SceneComponent.SetRelativeScale3D` (`self.Cube`) _new_scale_3d))))

(fn `UserConstructionScript`)