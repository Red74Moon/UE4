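; Game instance Blueprint that holds the score and level name and persists them through a BPSG_Score save object.
; SetScore only updates the held score, as its SaveGame call is disconnected.
; SaveGame writes that score and the current level's name to the fixed "SaveGame" slot.
; LoadGame reads a caller-specified slot and restores both values if the cast succeeds, without opening the level.
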(fn `LoadGame`
  (params (SlotName :type String) (UserIndex :type Integer))
  (bind _returnvalue (`GameplayStatics.LoadGameFromSlot` SlotName UserIndex))
  (bind _asbpsg_score (cast `/Game/Learn_Collision/BPSG_Score` _returnvalue))
  (set `self.SaveScore` (`/Game/Learn_Collision/BPSG_Score.Score` _asbpsg_score))
  (set `self.LevelName` (`/Game/Learn_Collision/BPSG_Score.LevelName` _asbpsg_score)))

(fn `SaveGame`
  (bind _returnvalue (`GameplayStatics.CreateSaveGameObject` "/Game/Learn_Collision/BPSG_Score.BPSG_Score_C"))
  (set `/Game/Learn_Collision/BPSG_Score.Score` (`self.SaveScore`) _returnvalue)
  (bind _returnvalue_2 (`GameplayStatics.GetCurrentLevelName` true))
  (bind _output_get (set `self.LevelName` (`KismetStringLibrary.Conv_StringToName` _returnvalue_2)))
  (set `/Game/Learn_Collision/BPSG_Score.LevelName` _output_get _returnvalue)
  (`GameplayStatics.SaveGameToSlot` _returnvalue "SaveGame"))

(fn `SetScore`
  (params (Score :type Integer))
  (set `self.SaveScore` Score))