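; BP_MoveRect is an actor in a collision learning folder that moves its Sphere component around a square loop in relative space.
; BeginPlay starts a looping 0.01-second timer on UpdateMoveRect, which switches on the MoveType state to call one of four directional move functions.
; Each function offsets the sphere along X or Y by Speed times a fixed step, then advances MoveType once the sphere passes that edge's limit.
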(event `self.ReceiveBeginPlay`
  (`KismetSystemLibrary.K2_SetTimer` null "UpdateMoveRect" 0.01 true))

(fn `MoveBottom`
  (params (DeltaSeconds :type "Float (double-precision)" :default 0.01))
  (bind (_relativelocation_x _relativelocation_y) (`KismetMathLibrary.BreakVector` (`SceneComponent.RelativeLocation` (`self.Sphere`))))
  (bind _result (`/Engine/EditorBlueprintResources/StandardMacros.NegateFloat` (* DeltaSeconds (`self.Speed`)))
    (:`  `
      (`SceneComponent.K2_AddRelativeLocation` (`self.Sphere`) (`KismetMathLibrary.MakeVector` 0.0 _result) false false)
      (if (< _relativelocation_y 0.0)
        (set `self.MoveType` "NewEnumerator0")))))

(fn `MoveLeft`
  (params (DeltaSeconds :type "Float (double-precision)" :default 0.01))
  (bind _relativelocation_x (`KismetMathLibrary.BreakVector` (`SceneComponent.RelativeLocation` (`self.Sphere`))))
  (bind _result (`/Engine/EditorBlueprintResources/StandardMacros.NegateFloat` (* DeltaSeconds (`self.Speed`)))
    (:`  `
      (`SceneComponent.K2_AddRelativeLocation` (`self.Sphere`) (`KismetMathLibrary.MakeVector` _result) false false)
      (if (< _relativelocation_x 0.0)
        (set `self.MoveType` "NewEnumerator3")))))

(fn `MoveRight`
  (params (DeltaSeconds :type "Float (double-precision)" :default 0.01))
  (bind _relativelocation_x (`KismetMathLibrary.BreakVector` (`SceneComponent.RelativeLocation` (`self.Sphere`))))
  (`SceneComponent.K2_AddRelativeLocation` (`self.Sphere`) (`KismetMathLibrary.MakeVector` (* DeltaSeconds (`self.Speed`))) false false)
  (if (> _relativelocation_x 300.0)
    (set `self.MoveType` "NewEnumerator1")))

(fn `MoveTop`
  (params (DeltaSeconds :type "Float (double-precision)" :default 0.01))
  (bind (_relativelocation_x _relativelocation_y) (`KismetMathLibrary.BreakVector` (`SceneComponent.RelativeLocation` (`self.Sphere`))))
  (`SceneComponent.K2_AddRelativeLocation` (`self.Sphere`) (`KismetMathLibrary.MakeVector` 0.0 (* DeltaSeconds (`self.Speed`))) false false)
  (if (> _relativelocation_y 300.0)
    (set `self.MoveType` "NewEnumerator2")))

(fn `UpdateMoveRect`
  (switch `/Game/Learn_Collision/EN_MoveType` (`self.MoveType`)
    (:`NewEnumerator0`
      (`self.MoveRight` 0.01))
    (:`NewEnumerator1`
      (`self.MoveTop` 0.01))
    (:`NewEnumerator2`
      (`self.MoveLeft` 0.01))
    (:`NewEnumerator3`
      (`self.MoveBottom` 0.01))))

(fn `UserConstructionScript`)