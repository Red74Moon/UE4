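; BP_TextActor is a collision-learning actor that counts how many times the player character has entered its cube and shows that count on its widget.
; BeginPlay caches the widget component's user widget as ActorWidget.
; Each begin overlap by BP_MyCharacter increments Count and writes it into the widget's MyText variable.
; End overlap does nothing, and leftover unconnected nodes for clearing the text and setting shadow casting never run.
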(event `self.ReceiveBeginPlay`
  (bind _asactor_widget (cast `/Game/Learn_Collision/ActorWidget` (`WidgetComponent.GetUserWidgetObject` (`self.Widget`)))))

(event `self.Cube.OnComponentBeginOverlap`
  (params (OverlappedComponent :type "PrimitiveComponent Object Reference") (OtherActor :type "Actor Object Reference") (OtherComp :type "PrimitiveComponent Object Reference") (OtherBodyIndex :type Integer) (bFromSweep :type Boolean) (SweepResult :type "HitResult Structure (by ref)"))
  (cast `/Game/Learn_Collision/BP_MyCharacter` OtherActor)
  (bind _result (`/Engine/EditorBlueprintResources/StandardMacros.IncrementInt` (`self.Count`))
    (:`  `
      (bind _output_get (set `self.Count` _result))
      (set `/Game/Learn_Collision/ActorWidget.MyText` (`KismetTextLibrary.Conv_IntToText` _output_get) (stale `self.ReceiveBeginPlay` _asactor_widget)))))

(event `self.Cube.OnComponentEndOverlap`
  (params (OverlappedComponent :type "PrimitiveComponent Object Reference") (OtherActor :type "Actor Object Reference") (OtherComp :type "PrimitiveComponent Object Reference") (OtherBodyIndex :type Integer)))

(fn `UserConstructionScript`)