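; BP_Qube is a collision-learning cube actor that demonstrates component overlap events with the player character.
; Its Cube component's begin and end overlap events respond only when the other actor casts to BP_MyCharacter.
; Each event prints its parameters to the screen for inspection and swaps the cube's material, one on entering and another on leaving.
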(event `self.Cube.OnComponentBeginOverlap`
  (params (OverlappedComponent :type "PrimitiveComponent Object Reference") (OtherActor :type "Actor Object Reference") (OtherComp :type "PrimitiveComponent Object Reference") (OtherBodyIndex :type Integer) (bFromSweep :type Boolean) (SweepResult :type "HitResult Structure (by ref)"))
  ;[1 1 1] Begin Overlap 출력내용 알아보기 / 큐브 머터리얼 바꾸기
  (cast `/Game/Learn_Collision/BP_MyCharacter` OtherActor)
  (`KismetSystemLibrary.PrintString` (`KismetStringLibrary.Concat_StrStr` "-- BeginOverLap Overlapped Component : " (`KismetSystemLibrary.GetDisplayName` OverlappedComponent) " \n-- BeginOverLap Other Actor : " (`KismetSystemLibrary.GetDisplayName` OtherActor) " \n-- BeginOverLap Other Comp : " (`KismetSystemLibrary.GetDisplayName` OtherComp) " \n-- BeginOverLap Sweep : " (`KismetStringLibrary.Conv_BoolToString` bFromSweep)) true true (struct :`G` 0.66 :`B` 1.0 :`A` 1.0) 30.0)
  (`PrimitiveComponent.SetMaterial` (`self.Cube`) 0 "/Engine/BufferVisualization/Anisotropy.Anisotropy"))

(event `self.Cube.OnComponentEndOverlap`
  (params (OverlappedComponent :type "PrimitiveComponent Object Reference") (OtherActor :type "Actor Object Reference") (OtherComp :type "PrimitiveComponent Object Reference") (OtherBodyIndex :type Integer))
  ;[1 1 1] End Overlap 출력내용 알아보기 / 큐브 머터리얼 바꾸기
  (cast `/Game/Learn_Collision/BP_MyCharacter` OtherActor)
  (`KismetSystemLibrary.PrintString` (`KismetStringLibrary.Concat_StrStr` "-- EndOverLap Overlapped Component : " (`KismetSystemLibrary.GetDisplayName` OverlappedComponent) " \n-- EndOverLap Other Actor : " (`KismetSystemLibrary.GetDisplayName` OtherActor) " \n-- EndOverLap Other Comp : " (`KismetSystemLibrary.GetDisplayName` OtherComp) " \n-- EndOverLap Other Body Index : " (`KismetStringLibrary.Conv_IntToString` OtherBodyIndex)) true true (struct :`G` 0.66 :`B` 1.0 :`A` 1.0) 30.0)
  (`PrimitiveComponent.SetMaterial` (`self.Cube`) 0 "/Engine/MapTemplates/Materials/BasicAsset03.BasicAsset03"))

(fn `UserConstructionScript`)