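; BP_MoveActor is an actor whose Sphere component ping-pongs along its local X axis.
; Tick offsets the Sphere at a frame-rate-independent speed and flips IsRight when its relative X passes either fixed bound.
; A separate CountTimer function, not called in this graph, accumulates its input into TotalDist, prints a minutes-and-seconds string and shifts the whole actor along X.
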(event `self.ReceiveTick`
  (params (DeltaSeconds :type "Float (single-precision)"))
  (bind _returnvalue (* DeltaSeconds 100.0))
  (bind _sphere (`self.Sphere`))
  (bind _relativelocation_x (`KismetMathLibrary.BreakVector` (`SceneComponent.RelativeLocation` (`self.Sphere`))))
  (bind _relativelocation_x_2 (`KismetMathLibrary.BreakVector` (`SceneComponent.RelativeLocation` (`self.Sphere`))))
  (if (`self.IsRight`)
    (`SceneComponent.K2_AddLocalOffset` _sphere (`KismetMathLibrary.MakeVector` _returnvalue) false false)
    (if (> _relativelocation_x 200.0)
      (set `self.IsRight` false))
    (else
      (bind _result (`/Engine/EditorBlueprintResources/StandardMacros.NegateFloat` _returnvalue)
        (:`  `
          (`SceneComponent.K2_AddLocalOffset` _sphere (`KismetMathLibrary.MakeVector` _result) false false)
          (if (< _relativelocation_x_2 0.0)
            (set `self.IsRight` true)))))))

(fn `CountTimer`
  (params (A :type "Float (double-precision)"))
  (bind _returnvalue (* A 1.0))
  (bind _returnvalue_2 (+ _returnvalue (`self.TotalDist`)))
  (set `self.TotalDist` _returnvalue_2)
  (`KismetSystemLibrary.PrintString` (`KismetStringLibrary.Concat_StrStr` (`KismetStringLibrary.Conv_IntToString` (`KismetMathLibrary.FFloor` (/ _returnvalue_2 60.0))) "m" (`KismetStringLibrary.Conv_IntToString` (`KismetMathLibrary.FFloor` (mod _returnvalue_2 60.0))) "s"))
  (`self.K2_AddActorLocalOffset` (`KismetMathLibrary.MakeVector` _returnvalue)))

(fn `UserConstructionScript`)