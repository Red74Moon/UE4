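; BP_MyPawn is a player pawn that flies freely around the level with adjustable speed.
; MoveForward and MoveRight axes offset the actor along the camera manager's forward and right vectors, scaled by PlayerSpeed, with no sweep or delta-time scaling.
; LookUp and LookRight axes drive controller pitch and yaw.
; SpeedUp and SpeedDown presses step PlayerSpeed up or down, clamped to a fixed range.
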(event `self.ReceiveTick`
  (params (DeltaSeconds :type "Float (single-precision)")))

(event `InputAxis|MoveForward`
  (params (AxisValue :type "Float (single-precision)"))
  (`self.K2_AddActorWorldOffset` (* (`self.GetActorForwardVector` (`GameplayStatics.GetPlayerCameraManager` 0)) (* AxisValue (`self.PlayerSpeed`)))))

(event `InputAxis|MoveRight`
  (params (AxisValue :type "Float (single-precision)"))
  (`self.K2_AddActorWorldOffset` (* (`self.GetActorRightVector` (`GameplayStatics.GetPlayerCameraManager` 0)) (* AxisValue (`self.PlayerSpeed`)))))

(event `InputAction|SpeedUp`
  (params (Key :type "Key Structure"))
  (:`Pressed`
    (bind _output_get (set `self.PlayerSpeed` (+ (`self.PlayerSpeed`) 10.0)))
    (if (>= _output_get 100.0)
      (set `self.PlayerSpeed` 100.0))))

(event `InputAxis|LookUp`
  (params (AxisValue :type "Float (single-precision)"))
  (`self.AddControllerPitchInput` AxisValue))

(event `InputAction|SpeedDown`
  (params (Key :type "Key Structure"))
  (:`Pressed`
    (bind _output_get (set `self.PlayerSpeed` (- (`self.PlayerSpeed`) 10.0)))
    (if (<= _output_get 10.0)
      (set `self.PlayerSpeed` 10.0))))

(event `InputAxis|LookRight`
  (params (AxisValue :type "Float (single-precision)"))
  (`self.AddControllerYawInput` AxisValue))

(fn `UserConstructionScript`)