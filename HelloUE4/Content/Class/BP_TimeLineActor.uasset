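; BP_TimeLineActor is a timeline practice actor that slides its Sphere back and forth along relative X.
; Timeline 타임라인_1 scales its track into the X location, and on finish flips IsMoveRight to alternate Play and Reverse endlessly.
; PressP, noted as an interface event, toggles PlayTimeActor and StopTimeLineActor through IsTimeLineMove.
; Tick, BeginPlay and PressPKey are empty, and earlier timeline, toggle and Delay tests remain disconnected.
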(event `self.ReceiveTick`
  (params (DeltaSeconds :type "Float (single-precision)"))
  ;[1 1 1] Tick 이벤트로 구성
)

(event `self.ReceiveBeginPlay`
  ;[1 1 1] Delay를 사용해서  테스트
)

(event `PlayTimeActor`
  ;[1 1 1] CustomEvent를 만들어 BeginPlay 이벤트에 연결해서 실행
  (set `self.IsTimeLineMove` true)
  (if (`self.IsMoveRight`) :!label _label
    (bind (_direction `_새_트랙_0`) (`Timeline|타임라인_1` :!label _label_2)
      (:`Update`
        (`SceneComponent.K2_SetRelativeLocation` (`self.Sphere`) (`KismetMathLibrary.MakeVector` (* `_새_트랙_0` 300.0)) false false))
      (:`Finished`
        (set `self.IsMoveRight` (not (`self.IsMoveRight`)))
        (goto _label)))
    (else
      (goto _label_2 :!via `Reverse`))))

(event `StopTimeLineActor`
  ;[1 1 1] CustomEvent를 만들어 BeginPlay 이벤트에 연결해서 실행
  (set `self.IsTimeLineMove` false)
  (goto _label_2 :!via `Stop`))

(event `PressPKey`
  ;[1 1 1] toggle 커스텀 함수 구현
)

(event `/Game/Class/BPI_PressP.PressP`
  ;[1 1 1] 인터페이스로 구성
  (if (`self.IsTimeLineMove`)
    (`self.StopTimeLineActor`)
    (else
      (`self.PlayTimeActor`))))

(fn `UserConstructionScript`)