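; Player pawn that flies through a test scene and controls four demo motion actors it spawns on BeginPlay.
; The P key toggles MoveRect and BP_MoveActor through boolean flags, and calls PressP and MoveP on the timeline and rotating-ball actors.
; Mouse axes drive look, while camera-relative offsets move the pawn without sweep at a key-adjustable, clamped Speed.
; R/F vertical movement and debug prints are disconnected.
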(event `InputAction|P_Key`
  (params (Key :type "Key Structure"))
  (bind _move_rect (`self.Move_Rect`))
  ;[1 1 1] 액터 스폰 / P 키 입력시 움직임
  (:`Pressed`
    (set `/Game/Class/BP_MoveRect.IsPlay` (not (`/Game/Class/BP_MoveRect.IsPlay` _move_rect)) _move_rect)
    ;[1 1 1] 구체 움직임 'P'키
    (set `/Game/Class/BP_MoveActor.IsMove` (not (`/Game/Class/BP_MoveActor.IsMove` (stale `self.ReceiveBeginPlay` _returnvalue_2))) (stale `self.ReceiveBeginPlay` _returnvalue_2))
    ;[1 1 1] TimeLine 'P'키
    (`/Game/Class/BP_TimeLineActor.PressP` (`self.BP_TimeLineActor`))
    ;[1 1 1] 시계추 'P'키
    (`/Game/Class/BP_RotationBall.MoveP` (`self.BP_RotationBallActor`))))

(event `self.ReceiveBeginPlay`
  ;[1 1 1] 액터 스폰 / P 키 입력시 움직임
  (bind _returnvalue (`|SpawnActorFromClass` (`self.Move_Rect1`) (`KismetMathLibrary.MakeTransform` (0.0 0.0 100.0)) "Undefined" "OverrideRootScale" null null))
  (set `self.Move_Rect` _returnvalue)
  ;[1 1 1] 구체 움직임 'P'키
  (bind _returnvalue_2 (`|SpawnActorFromClass` "/Game/Class/BP_MoveActor.BP_MoveActor_C" (`KismetMathLibrary.MakeTransform` (0.0 0.0 0.0)) "Undefined" "OverrideRootScale" null 0.0 null))
  ;[1 1 1] TimeLine 'P'키
  (bind _returnvalue_3 (`|SpawnActorFromClass` "/Game/Class/BP_TimeLineActor.BP_TimeLineActor_C" (`KismetMathLibrary.MakeTransform` (0.0 0.0 0.0)) "Undefined" "OverrideRootScale" null null))
  (set `self.BP_TimeLineActor` _returnvalue_3)
  ;[1 1 1] 시계추 'P'키
  (bind _returnvalue_4 (`|SpawnActorFromClass` "/Game/Class/BP_RotationBall.BP_RotationBall_C" (`KismetMathLibrary.MakeTransform` (0.0 0.0 300.0)) "Undefined" "OverrideRootScale" null null))
  (set `self.BP_RotationBallActor` _returnvalue_4))

(event `Key|F`
  (params (Key :type "Key Structure")))

(event `Key|R`
  (params (Key :type "Key Structure")))

(event `InputAxis|AxisTest`
  (params (AxisValue :type "Float (single-precision)"))
  ;[1 1 1] 코멘트
)

(event `InputAxis|F_Key`
  (params (AxisValue :type "Float (single-precision)"))
  ;[1 1 1] R-F 위-아래 움직임
)

(event `InputAction|HelloWorld`
  (params (Key :type "Key Structure"))
  ;[1 1 1] 코멘트
)

(event `InputAxis|R_Key`
  (params (AxisValue :type "Float (single-precision)"))
  ;[1 1 1] R-F 위-아래 움직임
)

(event `InputAxis|LookUp`
  (params (AxisValue :type "Float (single-precision)"))
  ;[1 1 1] 마우스 움직임
  (`self.AddControllerPitchInput` AxisValue))

(event `InputAxis|LookRight`
  (params (AxisValue :type "Float (single-precision)"))
  ;[1 1 1] 마우스 움직임
  (`self.AddControllerYawInput` AxisValue))

(event `InputAxis|MoveForward`
  (params (AxisValue :type "Float (single-precision)"))
  ;[1 1 1] 앞 뒤 움직임
  (`self.K2_AddActorWorldOffset` (* (`self.GetActorForwardVector` (`GameplayStatics.GetPlayerCameraManager` 0)) (* AxisValue (`self.speed`)))))

(event `InputAction|SpeedUp`
  (params (Key :type "Key Structure"))
  ;[1 1 1] 카메라 줌인(1-key) 아웃(2-key)
  (:`Pressed`
    (bind _output_get (set `self.speed` (+ (`self.speed`) 10.0)))
    (if (> _output_get 100.0)
      (set `self.speed` 100.0))))

(event `InputAction|SpeedDown`
  (params (Key :type "Key Structure"))
  ;[1 1 1] 카메라 줌인(1-key) 아웃(2-key)
  (:`Pressed`
    (bind _output_get (set `self.speed` (- (`self.speed`) 10.0)))
    (if (< _output_get 10.0)
      (set `self.speed` 10.0))))

(event `InputAxis|MoveRight`
  (params (AxisValue :type "Float (single-precision)"))
  ;[1 1 1] 좌우 움직임
  (`self.K2_AddActorLocalOffset` (* (`self.GetActorRightVector` (`GameplayStatics.GetPlayerCameraManager` 0)) (* AxisValue (`self.speed`)))))

(fn `UserConstructionScript`)