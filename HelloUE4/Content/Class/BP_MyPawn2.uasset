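; Player pawn that flies freely with mouse look and camera-relative movement, and triggers level actors with the P key.
; Move speed steps up or down within clamped limits; MoveRight feeds the camera's world right vector into a local offset.
; BeginPlay caches every BPI_PressP implementer, and P sends each PressPMessage through the interface.
; R/F vertical movement is unwired, and older per-class array and cast-chain versions remain disconnected.
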(event `InputAxis|LookUp`
  (params (AxisValue :type "Float (single-precision)"))
  ;[1 1 1] 마우스 움직임
  (`self.AddControllerPitchInput` AxisValue))

(event `InputAxis|LookRight`
  (params (AxisValue :type "Float (single-precision)"))
  ;[1 1 1] 마우스 움직임
  (`self.AddControllerYawInput` AxisValue))

(event `InputAxis|MoveForward`
  (params (AxisValue :type "Float (single-precision)"))
  ;[1 1 1] 앞 뒤 움직임
  (`self.K2_AddActorWorldOffset` (* (`self.GetActorForwardVector` (`GameplayStatics.GetPlayerCameraManager` 0)) (* AxisValue (`self.speed`)))))

(event `InputAction|P_Key`
  (params (Key :type "Key Structure"))
  ;[1 1 1] 이렇게 사용하지 말고
)

(event `InputAxis|MoveRight`
  (params (AxisValue :type "Float (single-precision)"))
  ;[1 1 1] 좌우 움직임
  (`self.K2_AddActorLocalOffset` (* (`self.GetActorRightVector` (`GameplayStatics.GetPlayerCameraManager` 0)) (* AxisValue (`self.speed`)))))

(event `InputAction|SpeedUp`
  (params (Key :type "Key Structure"))
  ;[1 1 1] 이동 속도 변경 코드 / 카메라 줌인(1-key) 아웃(2-key)
  (:`Pressed`
    (bind _output_get (set `self.speed` (+ (`self.speed`) 10.0)))
    (if (> _output_get 100.0)
      (set `self.speed` 100.0))))

(event `self.ReceiveBeginPlay`
  ;[1 1 1] 인터페이스를 사용한 코드로 구현한다.
  (bind _outactors (`GameplayStatics.GetAllActorsOfClass` "/Script/Engine.Actor"))
  (for _array_element _outactors
    (if (`KismetSystemLibrary.DoesImplementInterface` _array_element "/Game/Class/BPI_PressP.BPI_PressP_C")
      (`KismetArrayLibrary.Array_Add` (`self.Actors`) _array_element))))

(event `InputAction|SpeedDown`
  (params (Key :type "Key Structure"))
  ;[1 1 1] 이동 속도 변경 코드 / 카메라 줌인(1-key) 아웃(2-key)
  (:`Pressed`
    (bind _output_get (set `self.speed` (- (`self.speed`) 10.0)))
    (if (< _output_get 10.0)
      (set `self.speed` 10.0))))

(event `InputAction|P_Key`
  (params (Key :type "Key Structure"))
  ;[1 1 1] 배열 'Actors'에 담긴 class를 꺼내와 원하는 액터와 맞는지 cast형 변환을 통해 확인을 하여 일치하면 실행한다.
)

(event `InputAction|P_Key`
  (params (Key :type "Key Structure"))
  ;[1 1 1] 인터페이스를 사용한 코드로 구현한다.
  (:`Pressed`
    (for _array_element (`self.Actors`)
      (if (`KismetSystemLibrary.DoesImplementInterface` _array_element "/Game/Class/BPI_PressP.BPI_PressP_C")
        (message `/Game/Class/BPI_PressP.PressP` _array_element)))))

(event `InputAction|P_Key`
  (params (Key :type "Key Structure"))
  ;[1 1 1] 각각 배열에 입력된 값을 For 로 돌려 실행을 한다.
  ;;[1 1 1] 코멘트
)

(event `InputAxis|F_Key`
  (params (AxisValue :type "Float (single-precision)"))
  ;[1 1 1] R-F 위-아래 움직임
)

(event `InputAxis|R_Key`
  (params (AxisValue :type "Float (single-precision)"))
  ;[1 1 1] R-F 위-아래 움직임
)

(fn `UserConstructionScript`)