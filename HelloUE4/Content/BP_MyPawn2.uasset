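; Player pawn that flies with mouse look and camera-relative movement, and toggles several kinds of test actors in the level.
; Speed keys step movement speed within a clamped range; strafing feeds the camera's world-space right vector into a local offset.
; BeginPlay gathers four actor classes into one Actors array, which the P key walks, casting each to toggle or trigger it.
; R/F vertical movement is unwired, and older per-class array logic remains disconnected.
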(event `InputAxis|LookUp`
  (params (AxisValue :type "Float (single-precision)"))
  ;[1 1 1] 마우스 움직임
  (`self.AddControllerPitchInput` AxisValue))

(event `InputAxis|LookRight`
  (params (AxisValue :type "Float (single-precision)"))
  ;[1 1 1] 마우스 움직임
  (`self.AddControllerYawInput` AxisValue))

(event `InputAxis|MoveForward`
  (params (AxisValue :type "Float (single-precision)"))
  ;[1 1 1] 앞 뒤 움직임
  (`self.K2_AddActorWorldOffset` (* (`self.GetActorForwardVector` (`GameplayStatics.GetPlayerCameraManager` 0)) (* AxisValue (`self.speed`)))))

(event `InputAction|P_Key`
  (params (Key :type "Key Structure"))
  ;[1 1 1] 이렇게 사용하지 말고
)

(event `InputAxis|MoveRight`
  (params (AxisValue :type "Float (single-precision)"))
  ;[1 1 1] 좌우 움직임
  (`self.K2_AddActorLocalOffset` (* (`self.GetActorRightVector` (`GameplayStatics.GetPlayerCameraManager` 0)) (* AxisValue (`self.speed`)))))

(event `self.ReceiveBeginPlay`
  ;[1 1 1] 코멘트
  (`|ExecutionSequence`
    (:`then_0`
      (bind _outactors (`GameplayStatics.GetAllActorsOfClass` "/Game/BP_MoveActor.BP_MoveActor_C"))
      (for _array_element _outactors
        (`KismetArrayLibrary.Array_Add` (`self.Actors`) _array_element)))
    (:`then_1`
      (bind _outactors_2 (`GameplayStatics.GetAllActorsOfClass` "/Game/BP_MoveRect.BP_MoveRect_C"))
      (for _array_element_2 _outactors_2
        (`KismetArrayLibrary.Array_Add` (`self.Actors`) _array_element_2)))
    (:`then_2`
      (bind _outactors_3 (`GameplayStatics.GetAllActorsOfClass` "/Game/BP_RotationBall.BP_RotationBall_C"))
      (for _array_element_3 _outactors_3
        (`KismetArrayLibrary.Array_Add` (`self.Actors`) _array_element_3)))
    (:`then_3`
      (bind _outactors_4 (`GameplayStatics.GetAllActorsOfClass` "/Game/BP_TimeLineActor.BP_TimeLineActor_C"))
      (for _array_element_4 _outactors_4
        (`KismetArrayLibrary.Array_Add` (`self.Actors`) _array_element_4)))))

(event `InputAction|SpeedUp`
  (params (Key :type "Key Structure"))
  ;[1 1 1] 이동 속도 변경 코드 / 카메라 줌인(1-key) 아웃(2-key)
  (:`Pressed`
    (bind _output_get (set `self.speed` (+ (`self.speed`) 10.0)))
    (if (> _output_get 100.0)
      (set `self.speed` 100.0))))

(event `InputAction|SpeedDown`
  (params (Key :type "Key Structure"))
  ;[1 1 1] 이동 속도 변경 코드 / 카메라 줌인(1-key) 아웃(2-key)
  (:`Pressed`
    (bind _output_get (set `self.speed` (- (`self.speed`) 10.0)))
    (if (< _output_get 10.0)
      (set `self.speed` 10.0))))

(event `InputAction|P_Key`
  (params (Key :type "Key Structure"))
  ;[1 1 1] 코멘트
)

(event `InputAction|P_Key`
  (params (Key :type "Key Structure"))
  ;[1 1 1] 코멘트
  (:`Pressed`
    (for _array_element (`self.Actors`)
      (bind _asbp_move_actor (cast `/Game/BP_MoveActor` _array_element)
        (:`then`
          (set `/Game/BP_MoveActor.IsMove` (not (`/Game/BP_MoveActor.IsMove` _asbp_move_actor)) _asbp_move_actor))
        (:`CastFailed`
          (bind _asbp_move_rect (cast `/Game/BP_MoveRect` _array_element)
            (:`then`
              (set `/Game/BP_MoveRect.IsPlay` (not (`/Game/BP_MoveRect.IsPlay` _asbp_move_rect)) _asbp_move_rect))
            (:`CastFailed`
              (bind _asbp_rotation_ball (cast `/Game/BP_RotationBall` _array_element)
                (:`then`
                  (`/Game/BP_RotationBall.MoveP` _asbp_rotation_ball))
                (:`CastFailed`
                  (bind _asbp_time_line_actor (cast `/Game/BP_TimeLineActor` _array_element))
                  (`/Game/BP_TimeLineActor.PressP` _asbp_time_line_actor))))))))))

(event `InputAxis|F_Key`
  (params (AxisValue :type "Float (single-precision)"))
  ;[1 1 1] R-F 위-아래 움직임
)

(event `InputAxis|R_Key`
  (params (AxisValue :type "Float (single-precision)"))
  ;[1 1 1] R-F 위-아래 움직임
)

(fn `UserConstructionScript`)