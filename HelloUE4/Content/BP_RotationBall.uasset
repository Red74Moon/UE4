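; BP_RotationBall is a clock pendulum actor that swings by rolling its Center component, toggled on and off through the PressP interface event.
; PlayTime runs a timeline scaled by 45 degrees, flipping IsMoveRight on each finish to alternate Play and Reverse in a loop without Tick.
; PlayTimeStop halts the timeline.
; UpdateAddRotation, a speed-based alternative, is uncalled here, and several disconnected earlier graphs remain.
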(event `self.ReceiveTick`
  (params (DeltaSeconds :type "Float (single-precision)"))
  ;[1 1 1] 시계 추
)

(event `PlayTime`
  ;[1 1 1] toggle 함수에 대한 이벤트 함수(Tick 사용하지 않고 함수로 호출)
  ;;[1 1 1] toggle Key
  (set `self.IsPlay` true)
  (if (`self.IsMoveRight`) :!label _label
    (bind (_direction _value) (`Timeline|타임라인_1` :!label _label_2)
      (:`Update`
        (`SceneComponent.K2_SetRelativeRotation` (`self.Center`) (`KismetMathLibrary.MakeRotator` (* _value 45.0)) false false))
      (:`Finished`
        (set `self.IsMoveRight` (not (`self.IsMoveRight`)))
        (goto _label)))
    (else
      (goto _label_2 :!via `Reverse`))))

(event `PlayTimeStop`
  ;[1 1 1] toggle 함수에 대한 이벤트 함수(Tick 사용하지 않고 함수로 호출)
  ;;[1 1 1] toggle Key
  (set `self.IsPlay` false)
  (goto _label_2 :!via `Stop`))

(event `MoveP`
  ;[1 1 1] toggle 함수
)

(event `Go_P`
  ;[1 1 1] P key눌렀을때
)

(event `/Game/BPI_PressP.PressP`
  ;[1 1 1] 인터페이스로 구성
  (if (`self.IsPlay`)
    (`self.PlayTimeStop`)
    (else
      (`self.PlayTime`))))

(fn `UpdateAddRotation`
  (params (A :type "Float (double-precision)"))
  (bind _center (`self.Center`))
  (bind _returnvalue (* A (`self.Speed`)))
  (bind _relativelocation_x (`KismetMathLibrary.BreakVector` (`SceneComponent.RelativeLocation` (`self.Center`))))
  (bind _relativelocation_x_2 (`KismetMathLibrary.BreakVector` (`SceneComponent.RelativeLocation` (`self.Center`))))
  (if (`self.IsMoveRight`)
    (`SceneComponent.K2_AddRelativeRotation` _center (`KismetMathLibrary.MakeRotator` _returnvalue) false false)
    (if (> _relativelocation_x 45.0)
      (set `self.IsMoveRight` false))
    (else
      (bind _result (`/Engine/EditorBlueprintResources/StandardMacros.NegateFloat` _returnvalue)
        (:`  `
          (`SceneComponent.K2_AddRelativeRotation` _center (`KismetMathLibrary.MakeRotator` _result) false false)
          (if (< _relativelocation_x_2 -45.0)
            (set `self.IsMoveRight` true)))))))

(fn `UserConstructionScript`)