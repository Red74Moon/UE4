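; BP_MyPawn is a free-flying pawn steered by mouse look and movement axes.
; Movement offsets the actor without sweep along the camera manager's forward and right vectors, scaled by an adjustable, clamped Speed.
; MoveRight applies its camera vector as a local offset, while MoveForward uses a world offset.
; Test-actor spawning, their P-key toggles, R/F vertical movement and debug prints are disconnected and never run.
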(event `InputAction|P_Key`
  (params (Key :type "Key Structure"))
  ;[1 1 1] 액터 스폰 / P 키 입력시 움직임
)

(event `self.ReceiveBeginPlay`
  ;[1 1 1] 액터 스폰 / P 키 입력시 움직임
)

(event `Key|F`
  (params (Key :type "Key Structure")))

(event `Key|R`
  (params (Key :type "Key Structure")))

(event `InputAxis|AxisTest`
  (params (AxisValue :type "Float (single-precision)"))
  ;[1 1 1] 코멘트
)

(event `InputAxis|F_Key`
  (params (AxisValue :type "Float (single-precision)"))
  ;[1 1 1] R-F 위-아래 움직임
)

(event `InputAction|HelloWorld`
  (params (Key :type "Key Structure"))
  ;[1 1 1] 코멘트
)

(event `InputAxis|R_Key`
  (params (AxisValue :type "Float (single-precision)"))
  ;[1 1 1] R-F 위-아래 움직임
)

(event `InputAxis|LookUp`
  (params (AxisValue :type "Float (single-precision)"))
  ;[1 1 1] 마우스 움직임
  (`self.AddControllerPitchInput` AxisValue))

(event `InputAxis|LookRight`
  (params (AxisValue :type "Float (single-precision)"))
  ;[1 1 1] 마우스 움직임
  (`self.AddControllerYawInput` AxisValue))

(event `InputAxis|MoveForward`
  (params (AxisValue :type "Float (single-precision)"))
  ;[1 1 1] 앞 뒤 움직임
  (`self.K2_AddActorWorldOffset` (* (`self.GetActorForwardVector` (`GameplayStatics.GetPlayerCameraManager` 0)) (* AxisValue (`self.speed`)))))

(event `InputAction|SpeedUp`
  (params (Key :type "Key Structure"))
  ;[1 1 1] 카메라 줌인(1-key) 아웃(2-key)
  (:`Pressed`
    (bind _output_get (set `self.speed` (+ (`self.speed`) 10.0)))
    (if (> _output_get 100.0)
      (set `self.speed` 100.0))))

(event `InputAction|SpeedDown`
  (params (Key :type "Key Structure"))
  ;[1 1 1] 카메라 줌인(1-key) 아웃(2-key)
  (:`Pressed`
    (bind _output_get (set `self.speed` (- (`self.speed`) 10.0)))
    (if (< _output_get 10.0)
      (set `self.speed` 10.0))))

(event `InputAxis|MoveRight`
  (params (AxisValue :type "Float (single-precision)"))
  ;[1 1 1] 좌우 움직임
  (`self.K2_AddActorLocalOffset` (* (`self.GetActorRightVector` (`GameplayStatics.GetPlayerCameraManager` 0)) (* AxisValue (`self.speed`)))))

(fn `UserConstructionScript`)