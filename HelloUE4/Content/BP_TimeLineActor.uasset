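; BP_TimeLineActor is a timeline test actor that slides its Sphere back and forth along its relative X axis.
; Each Tick plays or reverses a timeline based on IsMoveRight, and the timeline's Update scales its value into the sphere's X position.
; Finished logs a message and flips IsMoveRight to switch direction.
; A second, near-identical timeline chain is present but never runs.
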(event `self.ReceiveTick`
  (params (DeltaSeconds :type "Float (single-precision)"))
  ;[1 1 1] 코멘트
  (if (`self.IsMoveRight`)
    (bind (_direction _value) (`Timeline|타임라인_0` :`NewTime` 3.0 :!label _label)
      (:`Update`
        (`SceneComponent.K2_SetRelativeLocation` (`self.Sphere`) (`KismetMathLibrary.MakeVector` (* _value 300.0)) false false))
      (:`Finished`
        (`KismetSystemLibrary.PrintString` "TimeLine Finished" false)
        (set `self.IsMoveRight` (not (`self.IsMoveRight`)))))
    (else
      (goto _label :!via `Reverse`))))

(fn `UserConstructionScript`)